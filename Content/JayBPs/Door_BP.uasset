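; Door actor that lets the player open a door map widget with the E key while overlapping it.
; Begin and end overlap toggle input on the actor and whether the map can be pulled up.
; E creates the DoorMap widget with UI-only input and a visible cursor, or, if the map is up, removes all widgets and hides the cursor without resetting the input mode.
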(event `Key|E`
  (params (Key :type "Key Structure"))
  (bind _returnvalue (`GameplayStatics.GetPlayerController` 0))
  (:`Pressed`
    (if (`self.canPullUpMap`)
      (if (`self.isMapUp`)
        (`WidgetLayoutLibrary.RemoveAllWidgets`)
        (set `PlayerController.bShowMouseCursor` false _returnvalue)
        (else
          (bind _returnvalue_2 (`|CreateWidget` "/Game/Widgets/DoorMap_Widget.DoorMap_Widget_C"))
          (`UserWidget.AddToViewport` _returnvalue_2 0)
          (`WidgetBlueprintLibrary.SetInputMode_UIOnlyEx` _returnvalue null)
          (set `PlayerController.bShowMouseCursor` true _returnvalue)))
      (set `self.isMapUp` (not (`self.isMapUp`))))))

(event `self.ReceiveActorBeginOverlap`
  (params (OtherActor :type "Actor Object Reference"))
  (`self.EnableInput` (`GameplayStatics.GetPlayerController` 0))
  (set `self.canPullUpMap` true))

(event `self.ReceiveActorEndOverlap`
  (params (OtherActor :type "Actor Object Reference"))
  (`self.DisableInput` (`GameplayStatics.GetPlayerController` 0))
  (set `self.canPullUpMap` false))

(fn `UserConstructionScript`)