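; BP_VoidDoor is a level-transition door that only lets the player through if it has been unlocked.
; A trigger overlap enables and disables input, so E works only while something is inside the trigger.
; On E, it searches the game instance's UnlockedDoors for its DoorName.
; A match stores that name as the spawn door and opens ThirdPersonExampleMap; otherwise it prints "Locked".
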(event `self.Trigger.OnComponentBeginOverlap`
  (params (OverlappedComponent :type "PrimitiveComponent Object Reference") (OtherActor :type "Actor Object Reference") (OtherComp :type "PrimitiveComponent Object Reference") (OtherBodyIndex :type Integer) (bFromSweep :type Boolean) (SweepResult :type "HitResult Structure (by ref)"))
  (`self.EnableInput` (`GameplayStatics.GetPlayerController` 0)))

(event `Key|E`
  (params (Key :type "Key Structure"))
  (bind _doorname (`self.doorName`))
  (:`Pressed`
    (bind _asmy_game_instance (cast `/Game/Blueprints/GameInstancesAndSaves/MyGameInstance` (`GameplayStatics.GetGameInstance`)))
    (set `self.isAnUnlockedDoor` false)
    (for _array_element (`/Game/Blueprints/GameInstancesAndSaves/MyGameInstance.UnlockedDoors` _asmy_game_instance)
      (if (`KismetStringLibrary.EqualEqual_StrStr` _array_element _doorname)
        (set `self.isAnUnlockedDoor` true)
        (bind _output_get (set `/Game/Blueprints/GameInstancesAndSaves/MyGameInstance.spawnPlayerAtThisDoor` _doorname _asmy_game_instance))
        (`GameplayStatics.OpenLevel` "ThirdPersonExampleMap")))
    (if (not (`self.isAnUnlockedDoor`))
      (`KismetSystemLibrary.PrintString` "Locked"))))

(event `self.Trigger.OnComponentEndOverlap`
  (params (OverlappedComponent :type "PrimitiveComponent Object Reference") (OtherActor :type "Actor Object Reference") (OtherComp :type "PrimitiveComponent Object Reference") (OtherBodyIndex :type Integer))
  (`self.DisableInput` (`GameplayStatics.GetPlayerController` 0)))

(fn `UserConstructionScript`)