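; BP_DreamDoor is a named door that links levels to VoidArea and serves as a player spawn point.
; On BeginPlay, the door matching the game instance's SpawnPlayerAtThisDoor moves TobyGuy just above itself.
; Trigger overlap enables input and records the name once in UnlockedDoors; leaving disables input.
; Pressing E opens VoidArea; the loop over unlocked doors does nothing, as its PrintString is disconnected.
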(event `self.ReceiveBeginPlay`
  (bind (_returnvalue_x _returnvalue_y _returnvalue_z) (`KismetMathLibrary.BreakVector` (`self.K2_GetActorLocation` self)))
  ;[1 1 1] Spawns the player at the correct door. Each door asks "am I the door we want to spawn at" basically
  (bind _asmy_game_instance (cast `/Game/Blueprints/GameInstancesAndSaves/MyGameInstance` (`GameplayStatics.GetGameInstance`)))
  (if (`KismetStringLibrary.EqualEqual_StrStr` (`self.doorName`) (`/Game/Blueprints/GameInstancesAndSaves/MyGameInstance.spawnPlayerAtThisDoor` _asmy_game_instance))
    (bind _astoby_guy (cast `/Game/Blueprints/Characters/TobyGuy` (`GameplayStatics.GetPlayerCharacter` 0)))
    (`self.K2_SetActorLocation` _astoby_guy (`KismetMathLibrary.MakeVector` _returnvalue_x _returnvalue_y (+ _returnvalue_z 100.0)) false false)))

(event `self.Trigger.OnComponentBeginOverlap`
  (params (OverlappedComponent :type "PrimitiveComponent Object Reference") (OtherActor :type "Actor Object Reference") (OtherComp :type "PrimitiveComponent Object Reference") (OtherBodyIndex :type Integer) (bFromSweep :type Boolean) (SweepResult :type "HitResult Structure (by ref)"))
  (bind _doorname (`self.doorName`))
  ;[1 1 1] Enable Input
  (`self.EnableInput` (`GameplayStatics.GetPlayerController` 0))
  ;[1 1 1] If the name of this door is not already in the list of unlocked doors, add it. Without this the same name gets added multiple times
  (bind _asmy_game_instance (cast `/Game/Blueprints/GameInstancesAndSaves/MyGameInstance` (`GameplayStatics.GetGameInstance`)))
  (bind _unlockeddoors (`/Game/Blueprints/GameInstancesAndSaves/MyGameInstance.UnlockedDoors` _asmy_game_instance))
  (for _array_element _unlockeddoors
    (if (`KismetStringLibrary.EqualEqual_StrStr` _array_element _doorname)
      (set `self.isAlreadyInList` true)))
  (if (not (`self.isAlreadyInList`))
    (`KismetArrayLibrary.Array_Add` _unlockeddoors _doorname) ; we only want to add to the list if it hasn't been added yet
  ))

(event `self.Trigger.OnComponentEndOverlap`
  (params (OverlappedComponent :type "PrimitiveComponent Object Reference") (OtherActor :type "Actor Object Reference") (OtherComp :type "PrimitiveComponent Object Reference") (OtherBodyIndex :type Integer))
  ;[1 1 1] Disable Input
  (`self.DisableInput` (`GameplayStatics.GetPlayerController` 0)))

(event `Key|E`
  (params (Key :type "Key Structure"))
  ;[1 1 1] Pressing E within a door opens the void and prints the list of unlocked doors
  (:`Pressed`
    (`GameplayStatics.OpenLevel` "VoidArea")
    (bind _asmy_game_instance (cast `/Game/Blueprints/GameInstancesAndSaves/MyGameInstance` (`GameplayStatics.GetGameInstance`)))
    (for _array_element (`/Game/Blueprints/GameInstancesAndSaves/MyGameInstance.UnlockedDoors` _asmy_game_instance)
      _)))

(fn `UserConstructionScript`)