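; EarthProjectil is an earth projectile Blueprint under Tomes that damages what it hits and sets off a stun blast when destroyed.
; A Sphere overlap applies the Damage value to the other actor, then destroys the projectile.
; The Destroyed event applies full, no-falloff radial StunDamageType damage around the Sphere, so the blast follows any destruction, not only a hit.
; Tick and construction only call the parent class.
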(event `self.ReceiveDestroyed`
  (`GameplayStatics.ApplyRadialDamage` :`BaseDamage` 2.0 :`Origin` (`SceneComponent.K2_GetComponentLocation` (`self.Sphere`)) :`DamageRadius` 800.0 :`DamageTypeClass` "/Game/Blueprints/Tomes/StunDamageType.StunDamageType_C" :`DamageCauser` null :`InstigatedByController` null :`bDoFullDamage` true))

(event `self.Sphere.OnComponentBeginOverlap`
  (params (OverlappedComponent :type "PrimitiveComponent Object Reference") (OtherActor :type "Actor Object Reference") (OtherComp :type "PrimitiveComponent Object Reference") (OtherBodyIndex :type Integer) (bFromSweep :type Boolean) (SweepResult :type "HitResult Structure (by ref)"))
  (`GameplayStatics.ApplyDamage` OtherActor (`self.Damage`))
  (`self.K2_DestroyActor`))

(event `self.ReceiveTick`
  (params (DeltaSeconds :type "Float (single-precision)"))
  (`parent.ReceiveTick` DeltaSeconds))

(fn `UserConstructionScript`
  (`parent.UserConstructionScript`))