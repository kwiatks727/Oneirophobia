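; BaseTome is a spellbook pickup that the TobyGuy character collects and fires projectiles from.
; Its first Box overlap with TobyGuy adds it to YourTomes and attaches it to him, becoming CurrentTome if it is the first or hidden otherwise.
; Once held, Tick refills Mp up to a cap, even while hidden, and applies IsVisible to the Book.
; Shoot spends MpCost to spawn the Projectile class along the follow camera's aim.
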(event `self.ReceiveTick`
  (params (DeltaSeconds :type "Float (single-precision)"))
  (bind _book (`self.Book`))
  (bind _returnvalue (+ (`self.Mp`) (* DeltaSeconds 20.0)))
  ;[1 1 1] Checks to see if you have the book
  (if (`self.HasBook`)
    ;[1 1 1] Reffils MP
    (if (> _returnvalue 100.0)
      (set `self.Mp` 100.0)
      (else
        (set `self.Mp` _returnvalue)))
    ;[1 1 1] Changes Visibilty
    (if (`self.isVisible`)
      (`SceneComponent.SetVisibility` _book true false)
      (else
        (`SceneComponent.SetVisibility` _book false false)))))

(event `self.Box.OnComponentBeginOverlap`
  (params (OverlappedComponent :type "PrimitiveComponent Object Reference") (OtherActor :type "Actor Object Reference") (OtherComp :type "PrimitiveComponent Object Reference") (OtherBodyIndex :type Integer) (bFromSweep :type Boolean) (SweepResult :type "HitResult Structure (by ref)"))
  ;[1 1 1] Checks to see if player is inside box, then add it too the arraylist in character
  (bind _astoby_guy (cast `/Game/Blueprints/Characters/TobyGuy` OtherActor))
  (`/Engine/EditorBlueprintResources/StandardMacros.DoOnce` false
    (:`Completed`
      (bind _yourtomes (`/Game/Blueprints/Characters/TobyGuy.YourTomes` _astoby_guy))
      (`KismetArrayLibrary.Array_Add` _yourtomes self)
      (if (> (`KismetArrayLibrary.Array_Length` _yourtomes) 1)
        (set `self.isVisible` false)
        (else
          (set `/Game/Blueprints/Characters/TobyGuy.CurrentTome` self _astoby_guy)))
      (set `self.HasBook` true)
      (`self.K2_AttachToActor` _astoby_guy "None" "SnapToTarget" "SnapToTarget" "KeepWorld" false)
      (`SceneComponent.K2_SetRelativeLocationAndRotation` (`self.Book`) (25.0 0.0 20.0) (struct :`Pitch` -90.0) false false))))

(fn `Shoot`
  (bind _returnvalue (`GameplayStatics.GetPlayerCharacter` 0))
  (bind _returnvalue_2 (- (`self.Mp`) (`self.MpCost`)))
  (bind _returnvalue_location (`KismetMathLibrary.BreakTransform` (`self.GetTransform` _returnvalue)))
  (bind _astoby_guy (cast `/Game/Blueprints/Characters/TobyGuy` _returnvalue))
  (if (> _returnvalue_2 0.0)
    (`KismetSystemLibrary.PrintString` (`KismetStringLibrary.Conv_DoubleToString` _returnvalue_2))
    (set `self.Mp` _returnvalue_2)
    (bind _followcamera (`/Game/Blueprints/Characters/TobyGuy.FollowCamera` _astoby_guy))
    (`|SpawnActorFromClass` (`self.Projectile`) (`KismetMathLibrary.MakeTransform` (+ _returnvalue_location (* (`SceneComponent.GetForwardVector` _followcamera) 100.0)) (`SceneComponent.K2_GetComponentRotation` _followcamera)) "Undefined" "OverrideRootScale" null null)))

(fn `UserConstructionScript`)