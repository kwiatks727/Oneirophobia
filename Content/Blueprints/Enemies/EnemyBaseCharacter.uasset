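; Base enemy character with health, a camera-facing health bar, stun, burning and knockback, which drains the player's Sanity under a range check that sums signed position offsets.
; Tick runs a state machine that returns to the spawn point, chases the player until switching to Attack (not handled here), applies knockback or dies.
; Timed events set stun, fire and knockback; death spins and shrinks the actor, then spawns monster parts.
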(event `self.ReceiveBeginPlay`
  (set `self.idleLocation` (`self.K2_GetActorLocation`))
  (bind _asenemy_health (cast `/Game/Blueprints/Enemies/EnemyHealth` (`WidgetComponent.GetWidget` (`self.HealthBar`))))
  (set `self.HealthBarRef` _asenemy_health)
  (bind _output_get (set `/Game/Blueprints/Enemies/EnemyHealth.MaxHealth` (`self.healthPoints`) _asenemy_health))
  (set `/Game/Blueprints/Enemies/EnemyHealth.CurrentHealth` _output_get _asenemy_health))

(event `self.ReceiveAnyDamage`
  (params (Damage :type "Float (single-precision)") (DamageType :type "DamageType Object Reference") (InstigatedBy :type "Controller Object Reference") (DamageCauser :type "Actor Object Reference"))
  (if (== (`GameplayStatics.GetObjectClass` DamageType) "/Game/Blueprints/Tomes/StunDamageType.StunDamageType_C")
    (`KismetSystemLibrary.PrintString` "AmTrue")
    (`self.Stun` Damage))
  (bind _output_get (set `self.healthPoints` (- (`self.healthPoints`) Damage)))
  (`KismetSystemLibrary.PrintString` (`KismetStringLibrary.Conv_DoubleToString` _output_get)))

(event `self.ReceiveTick`
  (params (DeltaSeconds :type "Float (single-precision)"))
  (bind _returnvalue (`GameplayStatics.GetPlayerCharacter` 0))
  (bind _returnvalue_2 (`self.K2_GetActorLocation` (`GameplayStatics.GetPlayerCharacter` 0)))
  (bind (_returnvalue_x _returnvalue_y _returnvalue_z) (`KismetMathLibrary.BreakVector` (- (`self.K2_GetActorLocation`) (`self.K2_GetActorLocation` _returnvalue))))
  (`SceneComponent.K2_SetWorldRotation` (`self.HealthBar`) (`KismetMathLibrary.FindLookAtRotation` (`SceneComponent.K2_GetComponentLocation` (`self.HealthBar`)) (`PlayerCameraManager.GetCameraLocation` (`GameplayStatics.GetPlayerCameraManager` 0))) false false)
  (bind _asenemy_health (cast `/Game/Blueprints/Enemies/EnemyHealth` (`WidgetComponent.GetWidget` (`self.HealthBar`))))
  (bind _output_get (set `/Game/Blueprints/Enemies/EnemyHealth.CurrentHealth` (`self.healthPoints`) _asenemy_health))
  (`KismetSystemLibrary.PrintString` (`KismetStringLibrary.Conv_DoubleToString` _output_get))
  ;[1 1 1] Checks if they are within range and then removes sanity from the player if they are
  (bind _astoby_guy (cast `/Game/Blueprints/Characters/TobyGuy` _returnvalue))
  (if (<= (+ _returnvalue_x _returnvalue_y _returnvalue_z) (`self.SanityDrainRange`))
    (set `/Game/Blueprints/Characters/TobyGuy.Sanity` (- (`/Game/Blueprints/Characters/TobyGuy.Sanity` _astoby_guy) (* (`self.SanityDrain`) DeltaSeconds)) _astoby_guy))
  (if (`self.Burning`)
    (`GameplayStatics.ApplyDamage` self (* DeltaSeconds 5.0)))
  (if (<= (`self.healthPoints`) 0.0)
    (set `self.state` "NewEnumerator3"))
  ;[1 1 1] State Handling
  (switch `/Game/Blueprints/Enemies/EnemyState` (`self.state`)
    (:`NewEnumerator0`
      (`|AIMoveTo` self (`self.idleLocation`) null))
    (:`NewEnumerator1`
      ;;[1 1 1] The enemy chases after the player until the player is within range, and then the player is attacked.
      (`|AIMoveTo` self _returnvalue_2 null (`self.moveToAcceptanceRadius`)
        (:`OnSuccess`
          (set `self.state` "NewEnumerator2")
          (set `self.playerTarget` _returnvalue_2))))
    (:`NewEnumerator3`
      (`self.DeathAnimation` DeltaSeconds))
    (:`NewEnumerator9`
      (`self.K2_SetActorLocation` self (+ (`self.K2_GetActorLocation` self) (`self.knockBackDistance`)) false false))))

(event `Stun`
  (params (StunDuration :type "Float (double-precision)"))
  (set `self.state` "NewEnumerator8")
  (`KismetSystemLibrary.Delay` StunDuration)
  (set `self.state` "NewEnumerator1"))

(event `SetOnFire`
  (set `self.Burning` true)
  (`KismetSystemLibrary.Delay` 4.0)
  (set `self.Burning` false))

(event `KnockBack`
  (params (Direction :type "Vector Structure"))
  (set `self.state` "NewEnumerator9")
  (bind _output_get (set `self.knockBackDistance` (* Direction 10.0)))
  (`KismetSystemLibrary.Delay` 0.5)
  (set `self.state` "NewEnumerator1")
  (set `self.playerTarget` (`self.K2_GetActorLocation` (`GameplayStatics.GetPlayerCharacter` 0))))

(fn `DeathAnimation`
  (params (DeltaTime :type "Float (double-precision)"))
  (`self.K2_AddActorWorldRotation` (`KismetMathLibrary.MakeRotator` 0.0 0.0 (* DeltaTime 360.0)))
  (`self.SetActorScale3D` (- (`self.GetActorScale3D`) DeltaTime))
  (bind _returnvalue (`self.FullyShrunk`))
  (if _returnvalue
    (for _ (range (+ (`self.monsterParts`) 1))
      (`|SpawnActorFromClass` "/Game/Blueprints/Enemies/MonsterPart.MonsterPart_C" (`KismetMathLibrary.MakeTransform` (+ (`self.K2_GetActorLocation`) (* (`self.GetActorUpVector`) 50.0))) "Undefined" "OverrideRootScale" null null))
    (`self.K2_DestroyActor`)))

(fn `FullyShrunk`
  (returns (ReturnValue :type Boolean))
  (bind (_returnvalue_x _returnvalue_y _returnvalue_z) (`KismetMathLibrary.BreakVector` (`self.GetActorScale3D`)))
  (return (or (<= _returnvalue_x 0.0) (<= _returnvalue_y 0.0) (<= _returnvalue_z 0.0))))

(fn `UserConstructionScript`
  (bind _asenemy_health (cast `/Game/Blueprints/Enemies/EnemyHealth` (`WidgetComponent.GetWidget` (`self.HealthBar`))))
  (set `self.HealthBarRef` _asenemy_health)
  (bind _output_get (set `/Game/Blueprints/Enemies/EnemyHealth.MaxHealth` (`self.healthPoints`) _asenemy_health))
  (set `/Game/Blueprints/Enemies/EnemyHealth.CurrentHealth` _output_get _asenemy_health))