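; Flying Shantak enemy that always faces the player and moves by a per-tick state machine without sweeping.
; Idle drifts randomly, steering back toward its idle location when it strays.
; Aggro flies straight at the player, switching to Attack at close range.
; Attack uses DoOnce gates to deal damage and pick a random retreat point, lerps briefly toward it, then resets to Aggro; nothing here triggers Idle-to-Aggro.
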(event `self.ReceiveBeginPlay`
  (`parent.ReceiveBeginPlay`)
  (bind _output_get (set `self.wanderDirection` (* (`KismetMathLibrary.RandomUnitVector`) (`KismetMathLibrary.RandomFloatInRange` 1.0 2.0)))))

(event `self.ReceiveTick`
  (params (DeltaSeconds :type "Float (single-precision)"))
  (bind _returnvalue (`self.K2_GetActorLocation`))
  (bind (_returnvalue_x _returnvalue_y _returnvalue_z) (`KismetMathLibrary.BreakVector` (`self.K2_GetActorLocation` (`GameplayStatics.GetPlayerCharacter` 0))))
  (bind _returnvalue_2 (`self.K2_GetActorLocation` (`GameplayStatics.GetPlayerCharacter` 0)))
  (bind _returnvalue_3 (+ (`self.lerpProgress`) (`self.lerpRate`)))
  (`parent.ReceiveTick` DeltaSeconds)
  (`self.K2_SetActorRotation` (`KismetMathLibrary.FindLookAtRotation` (`SceneComponent.K2_GetComponentLocation` (`self.Mesh`)) (`self.K2_GetActorLocation` (`GameplayStatics.GetPlayerCharacter` 0))))
  (switch `/Game/Blueprints/Enemies/EnemyState` (`self.state`)
    (:`NewEnumerator0`
      (`self.K2_AddActorWorldOffset` (`self.wanderDirection`))
      (`KismetSystemLibrary.Delay` (`KismetMathLibrary.RandomFloatInRange` 0.25 1.0))
      (if (> (`KismetMathLibrary.Vector_Distance` (`self.idleLocation`) (`self.K2_GetActorLocation`)) 200.0)
        (set `self.wanderDirection` (`KismetMathLibrary.Normal` (`KismetMathLibrary.Conv_RotatorToVector` (`KismetMathLibrary.FindLookAtRotation` (`self.K2_GetActorLocation`) (`self.idleLocation`)))))
        (else
          (set `self.wanderDirection` (* (`KismetMathLibrary.RandomUnitVector`) (`KismetMathLibrary.RandomFloatInRange` 1.0 2.0))))))
    (:`NewEnumerator1`
      (`self.K2_AddActorWorldOffset` (* (`KismetMathLibrary.Conv_RotatorToVector` (`KismetMathLibrary.FindLookAtRotation` _returnvalue _returnvalue_2)) (`self.flyingSpeed`)))
      (if (< (`KismetMathLibrary.Vector_Distance` _returnvalue _returnvalue_2) 100.0)
        (set `self.state` "NewEnumerator2")))
    (:`NewEnumerator2`
      (`|ExecutionSequence`
        (:`then_0`
          (`/Engine/EditorBlueprintResources/StandardMacros.DoOnce` false :!label _label
            (:`Completed`
              (`GameplayStatics.ApplyDamage` (`GameplayStatics.GetPlayerCharacter` 0) (`self.damageAmount`)))))
        (:`then_1`
          (`/Engine/EditorBlueprintResources/StandardMacros.DoOnce` false :!label _label_2
            (:`Completed`
              (set `self.retreatPoint` (`KismetMathLibrary.MakeVector` (+ (.x (`self.K2_GetActorLocation`)) (`KismetMathLibrary.RandomFloatInRange` -1000.0 1000.0)) (+ (.y (`self.K2_GetActorLocation`)) (`KismetMathLibrary.RandomFloatInRange` -1000.0 1000.0)) (+ (.z (`self.K2_GetActorLocation`)) (`KismetMathLibrary.RandomFloatInRange` _returnvalue_z (+ _returnvalue_z 1000.0)))))
              (bind _output_get (set `self.lerpRate` (/ (`self.retreatSpeed`) (`KismetMathLibrary.Vector_Distance` (`self.retreatPoint`) (`self.K2_GetActorLocation`)))))
              (set `self.lerpProgress` 0.0))))
        (:`then_2`
          (`self.K2_SetActorLocation` (`KismetMathLibrary.VLerp` (`self.K2_GetActorLocation`) (`self.retreatPoint`) _returnvalue_3))
          (bind _output_get_2 (set `self.lerpProgress` _returnvalue_3))
          (if (> (`self.lerpProgress`) 0.1)
            (set `self.state` "NewEnumerator1")
            (`|ExecutionSequence`
              (:`then_0`
                (goto _label :!via `Reset`))
              (:`then_1`
                (goto _label_2 :!via `Reset`)))))))))

(fn `UserConstructionScript`
  (`parent.UserConstructionScript`))