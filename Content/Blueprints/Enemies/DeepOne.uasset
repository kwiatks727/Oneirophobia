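; DeepOne is an enemy Blueprint that adds a melee attack to its parent class and sets the parent's move-to acceptance radius on construction.
; Tick watches the State enum and, in its attack state, uses a DoOnce to run one timed swing at a time.
; After a short delay, HitBox sphere-traces along Arrow1 with debug drawing, damaging TobyGuy if hit.
; On a hit, a further delay precedes switching State and resetting the DoOnce.
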(event `self.ReceiveTick`
  (params (DeltaSeconds :type "Float (single-precision)"))
  (`parent.ReceiveTick` DeltaSeconds)
  (if (`|EnumEquality` (`self.state`) "NewEnumerator2")
    (`/Engine/EditorBlueprintResources/StandardMacros.DoOnce` false :!label _label
      (:`Completed`
        (`KismetSystemLibrary.Delay` 0.25)
        (bind _outhit (`self.HitBox`))
        (bind _astoby_guy (cast `/Game/Blueprints/Characters/TobyGuy` (`.HitActor` (`GameplayStatics.BreakHitResult` _outhit)))
          (:`then`
            (`GameplayStatics.ApplyDamage` _astoby_guy 1.0)
            (`KismetSystemLibrary.PrintString` "Ow!"))
          (:`CastFailed`
            _))
        (`KismetSystemLibrary.Delay` 0.75)
        (set `self.state` "NewEnumerator1")
        (goto _label :!via `Reset`)))))

(fn `HitBox`
  (returns (OutHit :type "HitResult Structure"))
  (bind _arrow1 (`self.Arrow1`))
  (bind _returnvalue (`SceneComponent.K2_GetComponentLocation` _arrow1))
  (bind _outhit (`KismetSystemLibrary.SphereTraceSingle` :`Start` _returnvalue :`End` (+ _returnvalue (* (`SceneComponent.GetForwardVector` _arrow1) (`ArrowComponent.ArrowLength` _arrow1))) :`Radius` 35.200001 :`TraceChannel` "TraceTypeQuery2" :`DrawDebugType` "ForDuration" :`DrawTime` 1.0))
  (return _outhit))

(fn `UserConstructionScript`
  (`parent.UserConstructionScript`)
  (set `self.moveToAcceptanceRadius` 100.0))